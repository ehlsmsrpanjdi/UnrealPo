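; BP_ModularCar is a modular car actor that hosts four wheels as child actor components.
; On BeginPlay, a shared CCarSet helper casts each child actor to BP_Wheel and passes it the CarMesh through CWheelSet.
; The wheel logic itself lives outside this Blueprint.
; The four WheelStart calls in the event graph are unconnected and never run.
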(event `self.ReceiveBeginPlay`
  (`self.C_CarSet` (`self.BP_Wheel`))
  (`self.C_CarSet` (`self.BP_Wheel1`))
  (`self.C_CarSet` (`self.BP_Wheel2`))
  (`self.C_CarSet` (`self.BP_Wheel3`)))

(fn `C_CarSet`
  (params (`타깃` :type "ChildActorComponent Object Reference"))
  (bind _asbp_wheel (cast `/Game/ModularCar/Module/BP_Wheel` (`ChildActorComponent.ChildActor` `타깃`)))
  (`/Game/ModularCar/Module/BP_Wheel.C_WheelSet` _asbp_wheel (`self.Car_Mesh`)))

(fn `UserConstructionScript`)